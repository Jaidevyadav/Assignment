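; Player pawn that represents the top six-hitter, showing a name and team material, and walks between boundary locations waving.
; BeginPlay loads DT_Players into PlayerData and adds a Scoreboard widget; the VaRest web request feeding RequestedData is disconnected.
; FindPlayerWithMaxScores, not called here, picks the highest Sixes entry and starts a looping timer that drives AI MoveTo through Locations.
; The construction script applies the name text and material.
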(event `self.ReceiveBeginPlay`
  (`|ExecutionSequence`
    (:`then_0`
      (`self.Set Data`))
    (:`then_1`
      (bind _returnvalue (`|CreateWidget` "/Game/Blueprint/Scoreboard.Scoreboard_C"))
      (`UserWidget.AddToViewport` _returnvalue 0))))

(event `Requested Data`
  (params (Request :type "VaRestRequestJSON Object Reference"))
  ;[1 1 1] Getting Data
  (bind _returnvalue (`VaRestRequestJSON.GetResponseContentAsString` Request true))
  ;[1 1 1] Processing Data based on team, then storing it in array.
  (for _array_element (`KismetStringLibrary.ParseIntoArray` _returnvalue "*")
    (if (`KismetStringLibrary.EqualEqual_StrStr` _array_element (`|GetEnumeratorNameAsString` (`self.EnumTeam`)))
      (bind _returnvalue_2 (`KismetStringLibrary.Conv_StringToInt` _array_element))
      (`KismetArrayLibrary.Array_Add` (`self.PlayerData`) (make `/Game/Blueprint/Struct_PlayerData` "NewEnumerator0" _array_element _returnvalue_2))
      (else
        (`KismetArrayLibrary.Array_Add` (`self.PlayerData`) (make `/Game/Blueprint/Struct_PlayerData` "NewEnumerator0" _array_element _returnvalue_2))))))

(event `Call_To_Move_Event`
  ;[1 1 1] After processing Data it will move player to boundary
  (`KismetSystemLibrary.K2_SetTimerDelegate` (delegate `MovePlayer`) 5.0 true))

(event `MovePlayer`
  (bind _locations (`self.Locations`))
  (bind _index (`self.Index`))
  (bind _output (`|GetArrayItem` _locations (`self.Index`)))
  ;[1 1 1] After processing Data it will move player to boundary
  (if (`KismetArrayLibrary.Array_IsValidIndex` _locations)
    (`KismetSystemLibrary.PrintString` (`KismetSystemLibrary.GetDisplayName` _output))
    (`|AIMoveTo` self (0.0 0.0 0.0) _output
      (:`OnSuccess`
        (set `self.Wave` true)
        (`KismetSystemLibrary.Delay` 1.0)
        (set `self.Wave` false)
        (if (not (== (`KismetArrayLibrary.Array_Length` (`self.Locations`)) _index))
          (set `self.Index` (+ _index 1)))))))

(fn `Find Player With Max Scores`
  (locals (`Temp Value` :type Integer :default 1))
  (for _array_element (`self.PlayerData`)
    (bind (_team _name _sixes) (break `/Game/Blueprint/Struct_PlayerData` _array_element))
    (if (> _sixes (`local.Temp Value`))
      (set `local.Temp Value` _sixes)
      (set `self.Player With Highest Score` _name)
      (set `self.Team` _team)))
  (`self.Call_To_Move_Event`))

(fn `Set Data`
  (bind _outrownames (`DataTableFunctionLibrary.GetDataTableRowNames` "/Game/Blueprint/DT_Players.DT_Players"))
  (for _array_element _outrownames
    (bind _returnvalue (`|GetDataTableRow` "/Game/Blueprint/DT_Players.DT_Players" _array_element)
      (:`then`
        (bind _returnvalue_2 (`KismetArrayLibrary.Array_Add` (`self.PlayerData`) _returnvalue))
        (`KismetSystemLibrary.PrintString` (`KismetStringLibrary.Conv_IntToString` _returnvalue_2))))))

(fn `UserConstructionScript`
  (`TextRenderComponent.K2_SetText` (`self.TextRender`) (`KismetTextLibrary.Conv_StringToText` (`self.Player With Highest Score`)))
  (`PrimitiveComponent.SetMaterial` (`self.Mesh`) 0 (`self.Material`)))